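; BP_MyFloatingItem is a collectable item that the player picks up by pressing E while near it.
; Overlapping its Box with a TPPCharacter enables input from player controller 0 on the actor, and leaving disables it.
; Pressing E decrements CollectablesLeft on BP_OSPGameModeBase, adds a new Collectable_widget to the viewport and destroys the item.
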(event OnComponentBeginOverlap(Box)
  (params (OverlappedComponent :type Primitive%20Component%20Object%20Reference) (OtherActor :type Actor%20Object%20Reference) (OtherComp :type Primitive%20Component%20Object%20Reference) (OtherBodyIndex :type Integer) (bFromSweep :type Boolean) (SweepResult :type Hit%20Result%20Structure%20%28by%20ref%29))
  (Utilities|Casting|CastToTPPCharacter OtherActor)
  (Input|EnableInput (Game|GetPlayerController 0)))

(event OnComponentEndOverlap(Box)
  (params (OverlappedComponent :type Primitive%20Component%20Object%20Reference) (OtherActor :type Actor%20Object%20Reference) (OtherComp :type Primitive%20Component%20Object%20Reference) (OtherBodyIndex :type Integer))
  (Utilities|Casting|CastToTPPCharacter OtherActor)
  (Input|DisableInput (Game|GetPlayerController 0)))

(event Input|KeyboardEvents|E
  (params (Key :type Key%20Structure :default "None"))
  (:Pressed
    (bind _asbp_ospgame_mode_base (Utilities|Casting|CastToBP_OSPGameModeBase (Game|GetGameMode)))
    (bind _result (Math|Integer|DecrementInt (Variables|/Game/Blueprints/BP_OSPGameModeBase.BP_OSPGameModeBase_C|GetCollectables%20left _asbp_ospgame_mode_base))
      (:%20%20
        (Variables|/Game/Blueprints/BP_OSPGameModeBase.BP_OSPGameModeBase_C|SetCollectables%20left _asbp_ospgame_mode_base _result)
        (bind _returnvalue (UserInterface|CreateWidget "/Game/Blueprints/Collectable_widget.Collectable_widget_C"))
        (UserInterface|Viewport|AddtoViewport _returnvalue 0)
        (Actor|DestroyActor)))))

(fn ConstructionScript)