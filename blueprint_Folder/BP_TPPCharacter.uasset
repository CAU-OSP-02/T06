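; BP_TPPCharacter is a character Blueprint that switches between first-person and third-person views and changes movement speed.
; The Toggle Perspective action drives a FlipFlop that swaps the active FPP and TPP cameras, enabling controller yaw rotation only in first person.
; Hard-coded Left Shift and R key events set CharacterMovement's max walk speed to a faster and a much faster rate, restoring walking speed on release.
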(event Input|ActionEvents|InputActionTogglePerspective
  (params (Key :type Key%20Structure :default "None"))
  (:Pressed
    (Utilities|FlowControl|FlipFlop
      (:A
        (Components|Activation|SetActive (Variables|Default|GetFPP%20camera) true false)
        (Components|Activation|SetActive (Variables|Default|GetTPPCamera) false false)
        (Variables|Default|SetbUseControllerRotationYaw true))
      (:B
        (Components|Activation|SetActive (Variables|Default|GetFPP%20camera) false false)
        (Components|Activation|SetActive (Variables|Default|GetTPPCamera) true false)
        (Variables|Default|SetbUseControllerRotationYaw false)))))

(event Input|KeyboardEvents|LeftShift
  (params (Key :type Key%20Structure :default "None"))
  (bind _charactermovement (Variables|Character|GetCharacterMovement))
  (:Pressed
    (Variables|/Script/Engine.CharacterMovementComponent|SetMaxWalkSpeed _charactermovement 4e+02))
  (:Released
    (Variables|/Script/Engine.CharacterMovementComponent|SetMaxWalkSpeed _charactermovement 1.5e+02)))

(event Input|KeyboardEvents|R
  (params (Key :type Key%20Structure :default "None"))
  (bind _charactermovement (Variables|Character|GetCharacterMovement))
  (:Pressed
    (Variables|/Script/Engine.CharacterMovementComponent|SetMaxWalkSpeed _charactermovement 2e+03))
  (:Released
    (Variables|/Script/Engine.CharacterMovementComponent|SetMaxWalkSpeed _charactermovement 1.5e+02)))

(fn ConstructionScript)